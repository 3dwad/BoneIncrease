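; BP_Bullet is a bullet actor that applies its effects to whatever its sphere component first hits.
; The hit event runs once through a DoOnce, stores the hit actor and result, then calls two interface-checked functions.
; TryApplyDamage sends damage and the bullet's forward vector through BPI_Damage.
; TryIncreaseBone passes the hit bone name through BPI_ScaleIncraser to increase that bone.
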(event `self.Sphere.OnComponentHit`
  (params (HitComponent :type "PrimitiveComponent Object Reference") (OtherActor :type "Actor Object Reference") (OtherComp :type "PrimitiveComponent Object Reference") (NormalImpulse :type "Vector Structure") (Hit :type "HitResult Structure (by ref)"))
  (`/Engine/EditorBlueprintResources/StandardMacros.DoOnce` false
    (:`Completed`
      (set `self.HitActor` OtherActor)
      (set `self.HitResult` Hit)
      (`self.TryApplyDamage`)
      (`self.TryIncreaseBone`))))

(fn `TryApplyDamage`
  (if (`KismetSystemLibrary.DoesImplementInterface` (`self.HitActor`) "/Game/TZ/Interfaces/BPI_Damage.BPI_Damage_C")
    (message `/Game/TZ/Interfaces/BPI_Damage.ApplyDamage_BPI` (`self.HitActor`) (`self.Damage`) (`self.GetActorForwardVector`))))

(fn `TryIncreaseBone`
  (if (`KismetSystemLibrary.DoesImplementInterface` (`self.HitActor`) "/Game/TZ/Interfaces/BPI_ScaleIncraser.BPI_ScaleIncraser_C")
    (message `/Game/TZ/Interfaces/BPI_ScaleIncraser.IncreaseBone_BPI` (`self.HitActor`) (`.HitBoneName` (`GameplayStatics.BreakHitResult` (`self.HitResult`))))))

(fn `UserConstructionScript`)