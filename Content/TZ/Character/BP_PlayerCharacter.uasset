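; Player character Blueprint that fires BP_Bullet projectiles toward the point the follow camera is aiming at.
; The Shoot input runs a visibility line trace forward from the camera, using the impact point or the trace end as the target.
; The direction from ArrowForBullet to that target orients the spawned bullet, correcting for the offset between camera and muzzle.
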(event `InputAction|Shoot`
  (params (Key :type "Key Structure"))
  (bind _followcamera (`self.FollowCamera`))
  (bind _returnvalue (`SceneComponent.K2_GetComponentLocation` _followcamera))
  (:`Pressed`
    (bind (_outhit _returnvalue_2) (`KismetSystemLibrary.LineTraceSingle` _returnvalue (+ _returnvalue (* (`SceneComponent.GetForwardVector` _followcamera) 3000.0)) "TraceTypeQuery1" true))
    (if _returnvalue_2
      (bind (_bblockinghit _binitialoverlap _time _distance _location _impactpoint _normal _impactnormal _physmat _hitactor _hitcomponent _hitbonename _hititem _faceindex _tracestart _traceend) (`GameplayStatics.BreakHitResult` _outhit))
      (set `self.ShootDirection` (`KismetMathLibrary.GetDirectionUnitVector` (`SceneComponent.K2_GetComponentLocation` (`self.ArrowForBullet`)) _impactpoint))
      (else
        (set `self.ShootDirection` (`KismetMathLibrary.GetDirectionUnitVector` (`SceneComponent.K2_GetComponentLocation` (`self.ArrowForBullet`)) _traceend))))
    (`self.SpawnBullet`)))

(event `SpawnBullet`
  (`|SpawnActorFromClass` "/Game/TZ/GameplayActors/BP_Bullet.BP_Bullet_C" (`KismetMathLibrary.MakeTransform` (`SceneComponent.K2_GetComponentLocation` (`self.ArrowForBullet`)) (`KismetMathLibrary.Conv_VectorToRotator` (`self.ShootDirection`))) "AlwaysSpawn" "OverrideRootScale" null null))

(fn `UserConstructionScript`)